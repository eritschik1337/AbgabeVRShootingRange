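; Enemy character that chases the VR player and destroys the player pawn when its mesh registers a hit.
; On BeginPlay it loads the saved high score into VRPawn, picks a random walk speed and loops AI MoveTo.
; Damage plays an explosion sound and halts movement, with a random montage before walking resumes.
; Death increments the player's kills, asynchronously saves any matched or beaten high score, and destroys the enemy.
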(event `self.ReceiveBeginPlay`
  (bind _slot_name (`self.Slot Name`))
  ;[1 1 1] Event Begin + Load Game Data (Highscore)
  (bind _asvrpawn (cast `/Game/VRTemplate/Blueprints/VRPawn` (`GameplayStatics.GetPlayerPawn` 0)))
  (bind _output_get (set `self.Char REF` _asvrpawn))
  (bind _returnvalue (`GameplayStatics.DoesSaveGameExist` _slot_name))
  (if _returnvalue
    (bind _returnvalue_2 (`GameplayStatics.LoadGameFromSlot` _slot_name))
    (bind _output_get_2 (set `self.SaverSubClass` _returnvalue_2))
    (bind _assave_game_hs (cast `/Game/VRTemplate/Blueprints/SaveGame_HS` _output_get_2))
    (set `/Game/VRTemplate/Blueprints/VRPawn.High Score` (`/Game/VRTemplate/Blueprints/SaveGame_HS.High Score` _assave_game_hs) (`self.Char REF`)))
  (`self.Chase Player` _output_get)
  (set `CharacterMovementComponent.MaxWalkSpeed` (select `int` (`KismetMathLibrary.RandomInteger` 3) :`0` 50.0 :`1` 150.0 :`2` 100.0 :`3` 200.0 :!type "Float (single-precision)") (`self.CharacterMovement`)))

(event `Chase Player`
  (params (`Player To Chase` :type "/Game/VRTemplate/Blueprints/VRPawn Object Reference"))
  ;[1 1 1] Chase Player
  (if (not (`self.isDead`))
    (`|AIMoveTo` self (0.0 0.0 0.0) `Player To Chase`
      (:`OnSuccess`
        _)
      (:`OnFail`
        _))
    (`self.Chase Player` (`self.Char REF`))))

(event `self.ReceiveAnyDamage`
  (params (Damage :type "Float (single-precision)") (DamageType :type "DamageType Object Reference") (InstigatedBy :type "Controller Object Reference") (DamageCauser :type "Actor Object Reference"))
  (bind _returnvalue (`self.K2_GetActorLocation`))
  (bind _slot_name (`self.Slot Name`))
  (bind _saversubclass (`self.SaverSubClass`))
  ;[1 1 1] Damage + Damage Sound + Kill Count + Save Game Data
  (if (not (`self.isDead`))
    (bind _output_get (set `self.Health` (`KismetMathLibrary.FClamp` (- (`self.Health`) Damage) 0.0 100.0)))
    (if (== _output_get 0.0)
      (`GameplayStatics.PlaySoundAtLocation` "/Game/StarterContent/Audio/Explosion_Cue.Explosion_Cue" _returnvalue (struct) 1.0 1.0 0.0 null null null null)
      (`CharacterMovementComponent.DisableMovement` (`self.CharacterMovement`))
      (set `self.isDead` true)
      (`|ExecutionSequence`
        (:`then_0`
          (bind _asvrpawn (cast `/Game/VRTemplate/Blueprints/VRPawn` (`GameplayStatics.GetPlayerPawn` 0)))
          (bind _kills (`/Game/VRTemplate/Blueprints/VRPawn.Kills` _asvrpawn))
          (`/Engine/EditorBlueprintResources/StandardMacros.IncrementInt` _kills
            (:`  `
              (if (>= _kills (`/Game/VRTemplate/Blueprints/VRPawn.High Score` _asvrpawn))
                (bind _output_get_2 (set `/Game/VRTemplate/Blueprints/VRPawn.High Score` _kills _asvrpawn))
                (bind _returnvalue_2 (`GameplayStatics.DoesSaveGameExist` (`self.Slot Name`)))
                (if _returnvalue_2
                  (bind _returnvalue_3 (`GameplayStatics.LoadGameFromSlot` (`self.Slot Name`)))
                  (bind _output_get_3 (set `self.SaverSubClass` _returnvalue_3))
                  (bind _assave_game_hs (cast `/Game/VRTemplate/Blueprints/SaveGame_HS` _output_get_3))
                  (set `/Game/VRTemplate/Blueprints/SaveGame_HS.High Score` _output_get_2 _assave_game_hs)
                  (`AsyncActionHandleSaveGame.AsyncSaveGameToSlot` _saversubclass _slot_name)
                  (else
                    (bind _returnvalue_4 (`GameplayStatics.CreateSaveGameObject` "/Game/VRTemplate/Blueprints/SaveGame_HS.SaveGame_HS_C"))
                    (bind _output_get_4 (set `self.SaverSubClass` _returnvalue_4))
                    (bind _assave_game_hs_2 (cast `/Game/VRTemplate/Blueprints/SaveGame_HS` _output_get_4))
                    (set `/Game/VRTemplate/Blueprints/SaveGame_HS.High Score` _output_get_2 _assave_game_hs_2)
                    (`AsyncActionHandleSaveGame.AsyncSaveGameToSlot` _saversubclass _slot_name)))))))
        (:`then_1`
          (`self.K2_DestroyActor`)))
      (else
        (`GameplayStatics.PlaySoundAtLocation` "/Game/StarterContent/Audio/Explosion_Cue.Explosion_Cue" _returnvalue (struct) 1.0 1.0 0.0 null null null null)
        (`CharacterMovementComponent.DisableMovement` (`self.CharacterMovement`))
        (bind _returnvalue_5 (`self.PlayAnimMontage` (select `int` (`KismetMathLibrary.RandomInteger` 3) :`0` null :`1` null :`2` null :`3` null :!type "AnimMontage Object Reference")))
        (`KismetSystemLibrary.Delay` _returnvalue_5)
        (if (not (`self.isDead`))
          (`CharacterMovementComponent.SetMovementMode` (`self.CharacterMovement`) "MOVE_Walking" 0))))))

(event `self.Mesh.OnComponentHit`
  (params (HitComponent :type "PrimitiveComponent Object Reference") (OtherActor :type "Actor Object Reference") (OtherComp :type "PrimitiveComponent Object Reference") (NormalImpulse :type "Vector Structure") (Hit :type "HitResult Structure (by ref)"))
  ;[1 1 1] Funktion Enemy trifft Spieler, Spieler wird weg teleportiert
  (cast `/Game/VRTemplate/Blueprints/VRPawn` (`self.Char REF`))
  (if true
    (`self.K2_DestroyActor` (`GameplayStatics.GetPlayerPawn` 0))
    (else
      (`KismetSystemLibrary.PrintString` "No Charactar"))))

(fn `UserConstructionScript`)